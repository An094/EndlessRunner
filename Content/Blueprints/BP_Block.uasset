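; Track block for an endless runner that randomizes obstacles, two buildings and a four-lane coin on BeginPlay.
; When enabled, coin flips assign random meshes to sidewalk and street obstacle slots.
; Tick drives the two street obstacles along -X at VehicleSpeed, and player overlap with any obstacle quits the game.
; Player overlap with the Overlap trigger asks the game mode to add a block, then destroys this one after a delay.
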(event `self.ReceiveBeginPlay`
  (`self.SpawnObstacle`)
  (`self.SpawnBuilding`)
  (`self.SpawnCoin`))

(event `self.ReceiveTick`
  (params (DeltaSeconds :type "Float (single-precision)"))
  (bind _obstacle3 (`self.Obstacle3`))
  (bind _obstacle2 (`self.Obstacle2`))
  (bind (_returnvalue_x _returnvalue_y _returnvalue_z) (`KismetMathLibrary.BreakVector` (`SceneComponent.K2_GetComponentLocation` _obstacle3)))
  (bind (_returnvalue_x_2 _returnvalue_y_2 _returnvalue_z_2) (`KismetMathLibrary.BreakVector` (`SceneComponent.K2_GetComponentLocation` _obstacle2)))
  (`|ExecutionSequence`
    (:`then_0`
      (`/Engine/EditorBlueprintResources/StandardMacros.IsValid` (`StaticMeshComponent.StaticMesh` _obstacle2)
        (:`Is Valid`
          (`SceneComponent.K2_SetWorldLocation` (`self.Obstacle2`) (`KismetMathLibrary.MakeVector` (- _returnvalue_x_2 (* DeltaSeconds (`self.VehicleSpeed`))) _returnvalue_y_2 _returnvalue_z_2) false false))))
    (:`then_1`
      (`/Engine/EditorBlueprintResources/StandardMacros.IsValid` (`StaticMeshComponent.StaticMesh` _obstacle3)
        (:`Is Valid`
          (`SceneComponent.K2_SetWorldLocation` (`self.Obstacle3`) (`KismetMathLibrary.MakeVector` (- _returnvalue_x (* DeltaSeconds (`self.VehicleSpeed`))) _returnvalue_y _returnvalue_z) false false))))))

(event `self.Overlap.OnComponentBeginOverlap`
  (params (OverlappedComponent :type "PrimitiveComponent Object Reference") (OtherActor :type "Actor Object Reference") (OtherComp :type "PrimitiveComponent Object Reference") (OtherBodyIndex :type Integer) (bFromSweep :type Boolean) (SweepResult :type "HitResult Structure (by ref)"))
  (cast `/Game/ThirdPersonBP/Blueprints/ThirdPersonCharacter` OtherActor)
  (bind _asthird_person_game_mode (cast `/Game/ThirdPersonBP/Blueprints/ThirdPersonGameMode` (`GameplayStatics.GetGameMode`)))
  (`/Game/ThirdPersonBP/Blueprints/ThirdPersonGameMode.AddBlock` _asthird_person_game_mode true)
  (`KismetSystemLibrary.Delay` 5.0)
  (`self.K2_DestroyActor`))

(event `self.Obstacle1.OnComponentBeginOverlap`
  (params (OverlappedComponent :type "PrimitiveComponent Object Reference") (OtherActor :type "Actor Object Reference") (OtherComp :type "PrimitiveComponent Object Reference") (OtherBodyIndex :type Integer) (bFromSweep :type Boolean) (SweepResult :type "HitResult Structure (by ref)"))
  (cast `/Game/ThirdPersonBP/Blueprints/ThirdPersonCharacter` OtherActor)
  (`KismetSystemLibrary.QuitGame` null "Quit"))

(event `self.Obstacle2.OnComponentBeginOverlap`
  (params (OverlappedComponent :type "PrimitiveComponent Object Reference") (OtherActor :type "Actor Object Reference") (OtherComp :type "PrimitiveComponent Object Reference") (OtherBodyIndex :type Integer) (bFromSweep :type Boolean) (SweepResult :type "HitResult Structure (by ref)"))
  (cast `/Game/ThirdPersonBP/Blueprints/ThirdPersonCharacter` OtherActor)
  (`KismetSystemLibrary.QuitGame` null "Quit"))

(event `self.Obstacle3.OnComponentBeginOverlap`
  (params (OverlappedComponent :type "PrimitiveComponent Object Reference") (OtherActor :type "Actor Object Reference") (OtherComp :type "PrimitiveComponent Object Reference") (OtherBodyIndex :type Integer) (bFromSweep :type Boolean) (SweepResult :type "HitResult Structure (by ref)"))
  (cast `/Game/ThirdPersonBP/Blueprints/ThirdPersonCharacter` OtherActor)
  (`KismetSystemLibrary.QuitGame` null "Quit"))

(event `self.Obstacle4.OnComponentBeginOverlap`
  (params (OverlappedComponent :type "PrimitiveComponent Object Reference") (OtherActor :type "Actor Object Reference") (OtherComp :type "PrimitiveComponent Object Reference") (OtherBodyIndex :type Integer) (bFromSweep :type Boolean) (SweepResult :type "HitResult Structure (by ref)"))
  (cast `/Game/ThirdPersonBP/Blueprints/ThirdPersonCharacter` OtherActor)
  (`KismetSystemLibrary.QuitGame` null "Quit"))

(fn `SpawnBuilding`
  (`|ExecutionSequence`
    (:`then_0`
      (`StaticMeshComponent.SetStaticMesh` (`self.Building1`) (`KismetArrayLibrary.Array_Random` (`self.BuildingMeshes`))))
    (:`then_1`
      (`StaticMeshComponent.SetStaticMesh` (`self.Building2`) (`KismetArrayLibrary.Array_Random` (`self.BuildingMeshes`))))))

(fn `SpawnCoin`
  (bind (_returnvalue_x _returnvalue_y _returnvalue_z) (`KismetMathLibrary.BreakVector` (`self.K2_GetActorLocation`)))
  (`|SpawnActorFromClass` "/Game/Blueprints/BP_Coin.BP_Coin_C" (`KismetMathLibrary.MakeTransform` (`KismetMathLibrary.MakeVector` _returnvalue_x (+ (+ _returnvalue_y 200.0) (* (`KismetMathLibrary.RandomIntegerInRange` 0 3) 400.0)) (+ _returnvalue_z 100.0))) "Undefined" "OverrideRootScale" null null))

(fn `SpawnObstacle`
  (if (`self.DoSpawnObstacle`)
    (if (== (`KismetMathLibrary.RandomIntegerInRange` 0 1) 0)
      (`|ExecutionSequence`
        (:`then_0`
          (if (== (`KismetMathLibrary.RandomIntegerInRange` 0 1) 0)
            (`StaticMeshComponent.SetStaticMesh` (`self.Obstacle1`) (`KismetArrayLibrary.Array_Random` (`self.SidewalkMeshes`)))))
        (:`then_1`
          (if (== (`KismetMathLibrary.RandomIntegerInRange` 0 1) 0)
            (`StaticMeshComponent.SetStaticMesh` (`self.Obstacle2`) (`KismetArrayLibrary.Array_Random` (`self.StreetMeshes`)))))
        (:`then_2`
          (if (== (`KismetMathLibrary.RandomIntegerInRange` 0 1) 0)
            (`StaticMeshComponent.SetStaticMesh` (`self.Obstacle3`) (`KismetArrayLibrary.Array_Random` (`self.StreetMeshes`)))))
        (:`then_3`
          (if (== (`KismetMathLibrary.RandomIntegerInRange` 0 1) 0)
            (`StaticMeshComponent.SetStaticMesh` (`self.Obstacle4`) (`KismetArrayLibrary.Array_Random` (`self.SidewalkMeshes`)))))))))

(fn `UserConstructionScript`)